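; Spawner that scatters weapon and magazine pickups at random spots within a spawn area on BeginPlay.
; It spawns one rifle-mesh weapon pickup for each of two weapon types, plus ten magazines of randomly chosen type.
; Locations come from a downward visibility trace from the top of random points in the area bounds, raised slightly off the hit.
; A missed trace retries recursively, with no attempt limit.
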(event EventBeginPlay
  (CallFunction|SpawnWeapons)
  (CallFunction|SpawnMagazines))

(fn ConstructionScript)

(fn GetRandomSpawnLocation
  (bind _spawnareamin (Variables|Default|GetSpawnAreaMin))
  (bind _spawnareamax (Variables|Default|GetSpawnAreaMax))
  (bind _returnvalue (Math|Random|RandomFloatinRange (.y _spawnareamin) (.y _spawnareamax)))
  (bind _returnvalue_2 (Math|Random|RandomFloatinRange (.x _spawnareamin) (.x _spawnareamax)))
  (bind _returnvalue_3 (Math|Vector|MakeVector _returnvalue_2 _returnvalue (.z _spawnareamax)))
  (bind (_outhit _returnvalue_4) (Collision|LineTraceByChannel _returnvalue_3 (- _returnvalue_3 "0.000000,0.000000,5000.000000") "TraceTypeQuery1" false 0 "None"))
  (if _returnvalue_4
    (return (Math|Transform|MakeTransform (+ (.Location (Collision|BreakHitResult _outhit)) "0.000000,0.000000,10.000000") "0, 0, 0" "1.000000,1.000000,1.000000"))
    (else
      (bind _location (CallFunction|GetRandomSpawnLocation))
      (return _location))))

(fn SpawnWeapons
  (bind _location (CallFunction|GetRandomSpawnLocation))
  (Game|SpawnActorfromClass "/Game/Blueprints/Player/Weapon/BP_PickupWeapon.BP_PickupWeapon_C" _location "Undefined" "MultiplyWithRoot" 0 (Utilities|Struct|MakeSTR_PickupData "NewEnumerator0" "/Game/Assets/Weapons_Free/Meshes/SM_rifle_001.SM_rifle_001" "NewEnumerator0") 0)
  (bind _location_2 (CallFunction|GetRandomSpawnLocation))
  (Game|SpawnActorfromClass "/Game/Blueprints/Player/Weapon/BP_PickupWeapon.BP_PickupWeapon_C" _location_2 "Undefined" "MultiplyWithRoot" 0 (Utilities|Struct|MakeSTR_PickupData "NewEnumerator0" "/Game/Assets/Weapons_Free/Meshes/SM_rifle_001.SM_rifle_001" "NewEnumerator1") 0))

(fn SpawnMagazines
  (for _index (range 0 9)
    (bind _location (CallFunction|GetRandomSpawnLocation))
    (Game|SpawnActorfromClass "/Game/Blueprints/Player/Weapon/BP_PickupMagazine.BP_PickupMagazine_C" _location "Undefined" "MultiplyWithRoot" 0 (Utilities|Struct|MakeSTR_PickupData "NewEnumerator1" "/Game/Assets/Weapons_Free/Meshes/SM_rifle_magazine_001.SM_rifle_magazine_001" (Utilities|Enum|ByteToEnumE_WeaponType (Math|Conversions|ToByte(Integer) (Math|Random|RandomIntegerinRange 0 1)))) 0)))