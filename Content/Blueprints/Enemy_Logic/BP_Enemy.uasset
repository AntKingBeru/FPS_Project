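; Enemy actor that smoothly turns to face player 0 every tick.
; LookAtPlayer lerps roll and yaw toward the look-at rotation by delta time times Speed, then fires a debug-drawn forward visibility trace whose result is unused.
; IsPlayerInRange compares a facing dot product, using the player-to-enemy direction, against Range but is not called here.
; An AIMoveTo chase toward the player is present but disconnected.
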(event EventBeginPlay)

(event Collision|EventActorBeginOverlap
  (params (OtherActor :type Actor%20Object%20Reference)))

(event EventTick
  (params (DeltaSeconds :type Float%20%28single-precision%29))
  (CallFunction|LookatPlayer DeltaSeconds))

(fn ConstructionScript)

(fn LookatPlayer
  (params (A :type Float%20%28double-precision%29))
  (bind _returnvalue (Transformation|GetActorRotation))
  (bind _returnvalue_2 (Game|Player|GetPlayerPawn 0))
  (bind _returnvalue_3 (Transformation|GetActorLocation))
  (bind _returnvalue_4 (Transformation|GetActorLocation))
  (bind _speed (Variables|Default|GetSpeed))
  (bind _returnvalue_5 (Transformation|GetActorLocation _returnvalue_2))
  (bind _returnvalue_6 (* A _speed))
  (bind _returnvalue_7 (Math|Rotator|FindLookatRotation _returnvalue_4 _returnvalue_5))
  (bind _returnvalue_8 (Math|Rotator|Lerp(Rotator) _returnvalue _returnvalue_7 _returnvalue_6 true))
  (Transformation|SetActorRotation (Math|Rotator|MakeRotator (.roll _returnvalue_8) 0.0 (.yaw _returnvalue_8)))
  (Collision|LineTraceByChannel _returnvalue_3 (+ _returnvalue_3 (* (Transformation|GetActorForwardVector) 5e+02)) "TraceTypeQuery1" false 0 "ForOneFrame"))

(fn IsPlayerinRange
  (return (> (Math|Vector|DotProduct (Transformation|GetActorForwardVector) (Math|Vector|Normalize (- (Transformation|GetActorLocation) (Transformation|GetActorLocation (Game|Player|GetPlayerPawn 0))))) (Variables|Default|GetRange))))