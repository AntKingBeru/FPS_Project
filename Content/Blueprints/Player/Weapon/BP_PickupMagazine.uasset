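; BP_PickupMagazine is an ammo pickup that gives bullets to the player on overlap.
; BeginPlay writes BulletCount to its text label, then randomizes it within a range set by Data's weapon type, so the label shows the pre-roll value.
; Overlapping a BP_PlayerCharacter loops over UnlockedWeapons values, calling PickupItem and DestroyActor for each true entry, regardless of weapon type and without breaking.
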(event OnComponentBeginOverlap(Collision)
  (params (OverlappedComponent :type Primitive%20Component%20Object%20Reference) (OtherActor :type Actor%20Object%20Reference) (OtherComp :type Primitive%20Component%20Object%20Reference) (OtherBodyIndex :type Integer) (bFromSweep :type Boolean) (SweepResult :type Hit%20Result%20Structure%20%28by%20ref%29))
  (bind _asbp_player_character (Utilities|Casting|CastToBP_PlayerCharacter OtherActor))
  (bind _values (Utilities|Map|Values (Variables|/Game/Blueprints/Player/BP_PlayerCharacter.BP_PlayerCharacter_C|GetUnlockedWeapons _asbp_player_character)))
  (for _array_element _values
    (if _array_element
      (Default|PickupItem _asbp_player_character (Variables|Default|GetData) (Variables|Default|GetBulletCount))
      (Actor|DestroyActor))))

(event EventBeginPlay
  (Rendering|Components|TextRender|SetText (Variables|Default|GetTextRender) (Utilities|Text|ToText(String) (Utilities|String|ToString(Integer) (Variables|Default|GetBulletCount))))
  (switch Utilities|FlowControl|Switch|SwitchonE_WeaponType (.weapontype (Variables|Default|GetData))
    (:NewEnumerator0
      (Variables|Default|SetBulletCount (Math|Random|RandomIntegerinRange 10 20)))
    (:NewEnumerator1
      (Variables|Default|SetBulletCount (Math|Random|RandomIntegerinRange 5 10))))
  (|CallParentFunction))

(fn ConstructionScript
  (|CallParentFunction))