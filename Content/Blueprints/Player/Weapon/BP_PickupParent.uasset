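; Base pickup actor for weapons that the player collects by walking over it.
; At BeginPlay it sets the mesh material to mark weak or strong rifles according to the weapon type in its Data.
; On collision overlap with BP_PlayerCharacter it passes Data and BulletCount to PickupItem, then destroys itself.
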(event OnComponentBeginOverlap(Collision)
  (params (OverlappedComponent :type Primitive%20Component%20Object%20Reference) (OtherActor :type Actor%20Object%20Reference) (OtherComp :type Primitive%20Component%20Object%20Reference) (OtherBodyIndex :type Integer) (bFromSweep :type Boolean) (SweepResult :type Hit%20Result%20Structure%20%28by%20ref%29))
  (bind _asbp_player_character (Utilities|Casting|CastToBP_PlayerCharacter OtherActor))
  (Default|PickupItem _asbp_player_character (Variables|Default|GetData) (Variables|Default|GetBulletCount))
  (Actor|DestroyActor))

(event EventBeginPlay
  (switch Utilities|FlowControl|Switch|SwitchonE_WeaponType (.weapontype (Variables|Default|GetData))
    (:NewEnumerator0
      (Rendering|Material|SetMaterial (Variables|Default|GetMesh) 0 "/Game/Materials/M_WeakWeapon.M_WeakWeapon"))
    (:NewEnumerator1
      (Rendering|Material|SetMaterial (Variables|Default|GetMesh) 0 "/Game/Materials/M_StrongWeapon.M_StrongWeapon"))))

(fn ConstructionScript)