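; Enemy AI that patrols random nearby navigable points, chases players it sees and takes damage until death.
; On sighting, it idles, lerps its rotation toward the player, waits, then uses a forward-vector dot product to choose chase or patrol.
; A retriggerable delay returns chases to walking patrol, while an EnemyData struct records each state.
; Damage updates a widget health bar, and death increments GM_Level kills before destroying the actor.
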(event OnSeePawn(PawnSensing)
  (params (Pawn :type Pawn%20Object%20Reference))
  ;[0.15 0.15 0.15 0.5] Chase Player
  (Variables|Default|SetEnemyData (Utilities|Struct|MakeSTR_EnemyData (.isdead? (Variables|Default|GetEnemyData)) (.health (Variables|Default|GetEnemyData)) "NewEnumerator0"))
  (Components|Animation|PlayAnimation (Variables|Character|GetMesh) "/Game/Blueprints/Enemy/Animations/Enemy_Idle.Enemy_Idle" true)
  (CallFunction|LookatPlayer (Utilities|Time|GetWorldDeltaSeconds))
  (Utilities|FlowControl|Delay 3.0)
  (if (CallFunction|IsPlayerinRange)
    (Variables|Default|SetEnemyData (Utilities|Struct|MakeSTR_EnemyData (.isdead? (Variables|Default|GetEnemyData)) (.health (Variables|Default|GetEnemyData)) "NewEnumerator2"))
    (Utilities|FlowControl|Sequence
      (:then_0
        (Utilities|FlowControl|DoOnce false
          (:Completed
            (Components|Animation|PlayAnimation (Variables|Character|GetMesh) "/Game/Blueprints/Enemy/Animations/Enemy_Run.Enemy_Run" true)
            (Variables|/Script/Engine.CharacterMovementComponent|SetMaxWalkSpeed (Variables|Character|GetCharacterMovement) 6e+02))))
      (:then_1
        (AI|AIMoveTo self "0, 0, 0" Pawn (Variables|Default|GetAcceptanceRadius) true
          (:then
            (Utilities|FlowControl|RetriggerableDelay 7.0)
            (Components|Animation|PlayAnimation (Variables|Character|GetMesh) "/Game/Blueprints/Enemy/Animations/Enemy_Walk.Enemy_Walk" true)
            (Variables|/Script/Engine.CharacterMovementComponent|SetMaxWalkSpeed (Variables|Character|GetCharacterMovement) 1.3e+02)
            (CallFunction|CanRunAgain)
            (CallFunction|MovetoRandomLocation)))))
    (else
      (CallFunction|CanRunAgain)
      (CallFunction|MovetoRandomLocation))))

(event Custom|MoveToRandomLocation
  ;[0.15 0.15 0.15 0.5] Random Patrol
  (Variables|Default|SetEnemyData (Utilities|Struct|MakeSTR_EnemyData (.isdead? (Variables|Default|GetEnemyData)) (.health (Variables|Default|GetEnemyData)) "NewEnumerator1"))
  (bind _randomlocation (Class|NavigationSystemV1|GetRandomLocationinNavigableRadius (Transformation|GetActorLocation) 1e+03 0 0))
  (AI|AIMoveTo self _randomlocation 0 (Variables|Default|GetAcceptanceRadius) true
    (:OnSuccess
      (CallFunction|MovetoRandomLocation))))

(event Custom|CanRunAgain
  ;[0.15 0.15 0.15 0.5] Chase Player
  (Utilities|FlowControl|DoOnce false) ; enters at Reset
)

(event Custom|Die
  (Components|Animation|PlayAnimation (Variables|Character|GetMesh) "/Game/Blueprints/Enemy/Animations/Enemy_Attack_Bare.Enemy_Attack_Bare" true)
  (bind _asgm_level (Utilities|Casting|CastToGM_Level (Game|GetGameMode)))
  (bind _result (Math|Integer|IncrementInt (Variables|/Game/Blueprints/GameModes/GM_Level.GM_Level_C|GetKills _asgm_level))
    (:%20%20
      (Variables|/Game/Blueprints/GameModes/GM_Level.GM_Level_C|SetKills _asgm_level _result)
      (Utilities|FlowControl|Delay 2.5)
      (Actor|DestroyActor))))

(event EventBeginPlay
  ;[0.15 0.15 0.15 0.5] Start Patrol
  (Variables|Default|SetEnemyData (Utilities|Struct|MakeSTR_EnemyData (.isdead? (Variables|Default|GetEnemyData)) (.health (Variables|Default|GetEnemyData)) "NewEnumerator1"))
  (CallFunction|MovetoRandomLocation))

(event Game|Damage|EventAnyDamage
  (params (Damage :type Float%20%28single-precision%29) (DamageType :type Damage%20Type%20Object%20Reference) (InstigatedBy :type Controller%20Object%20Reference) (DamageCauser :type Actor%20Object%20Reference))
  ;[0.15 0.15 0.15 0.5] Take Damage
  (bind _output_get (Variables|Default|SetCurrentHP (- (Variables|Default|GetCurrentHP) Damage)))
  (bind _asumg_health_bar (Utilities|Casting|CastToUMG_HealthBar (UserInterface|GetWidget (Variables|Default|GetHealthBar))))
  (Default|SetPercent _asumg_health_bar (/ (- (.health (Variables|Default|GetEnemyData)) _output_get) (.health (Variables|Default|GetEnemyData))))
  (if (<= (Variables|Default|GetCurrentHP) 0.0)
    (Variables|Default|SetEnemyData (Utilities|Struct|MakeSTR_EnemyData true (.health (Variables|Default|GetEnemyData)) "NewEnumerator3"))
    (CallFunction|Die)))

(fn ConstructionScript)

(fn LookatPlayer
  (params (A :type Float%20%28double-precision%29))
  (bind _returnvalue (Transformation|GetActorRotation))
  (bind _returnvalue_2 (Game|Player|GetPlayerPawn 0))
  (bind _returnvalue_3 (Transformation|GetActorLocation))
  (bind _returnvalue_4 (Transformation|GetActorLocation))
  (bind _speed (Variables|Default|GetSpeed))
  (bind _returnvalue_5 (Transformation|GetActorLocation _returnvalue_2))
  (bind _returnvalue_6 (* A _speed))
  (bind _returnvalue_7 (Math|Rotator|FindLookatRotation _returnvalue_4 _returnvalue_5))
  (bind _returnvalue_8 (Math|Rotator|Lerp(Rotator) _returnvalue _returnvalue_7 _returnvalue_6 true))
  (Transformation|SetActorRotation (Math|Rotator|MakeRotator (.roll _returnvalue_8) 0.0 (.yaw _returnvalue_8)))
  (Collision|LineTraceByChannel _returnvalue_3 (+ _returnvalue_3 (* (Transformation|GetActorForwardVector) 5e+02)) "TraceTypeQuery1" false 0 "ForOneFrame"))

(fn IsPlayerinRange
  (return (> (Math|Vector|DotProduct (Transformation|GetActorForwardVector) (Math|Vector|Normalize (- (Transformation|GetActorLocation) (Transformation|GetActorLocation (Game|Player|GetPlayerPawn 0))))) (Variables|Default|GetRange))))