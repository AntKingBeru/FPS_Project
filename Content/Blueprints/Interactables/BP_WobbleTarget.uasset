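; Shootable wobble target whose dummy tips over when it takes damage, then stands back up.
; A timeline drives the dummy's pitch, then plays in reverse after a brief delay to reset it.
; A DoOnce gate ignores further hits until the reverse finishes, using a flag to tell fall from reset.
; The construction script links the static base plate to the physics-enabled dummy with a physics constraint.
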(event Custom|ResetTarget
  (bind _newtrack_0 (Timeline|Fallover%20Timeline ReverseFromEnd)
    (:Update
      (Transformation|SetRelativeRotation (Variables|Default|GetDummy) (Math|Rotator|MakeRotator 0.0 _newtrack_0 0.0) false false))
    (:Finished
      (if (Variables|Default|GetIsTargetShot?)
        (Variables|Default|SetIsTargetShot? false)
        (Utilities|FlowControl|Delay 0.0125)
        (CallFunction|ResetTarget)
        (else
          (Utilities|FlowControl|DoOnce false) ; enters at Reset
        )))))

(event Game|Damage|EventAnyDamage
  (params (Damage :type Float%20%28single-precision%29) (DamageType :type Damage%20Type%20Object%20Reference) (InstigatedBy :type Controller%20Object%20Reference) (DamageCauser :type Actor%20Object%20Reference))
  (Utilities|FlowControl|DoOnce false :!label _label
    (:Completed
      (Variables|Default|SetIsTargetShot? true)
      (bind _newtrack_0 (Timeline|Fallover%20Timeline PlayFromStart)
        (:Update
          (Transformation|SetRelativeRotation (Variables|Default|GetDummy) (Math|Rotator|MakeRotator 0.0 _newtrack_0 0.0) false false))
        (:Finished
          (if (Variables|Default|GetIsTargetShot?)
            (Variables|Default|SetIsTargetShot? false)
            (Utilities|FlowControl|Delay 0.0125)
            (CallFunction|ResetTarget)
            (else
              (goto _label Reset))))))))

(fn ConstructionScript
  ;[0.15 0.15 0.15 0.5] Set a constraint between the base plate (no physics enabled) and the dummy (physics enabled)
  (Class|PhysicsConstraintComponent|SetConstrainedComponents (Variables|Default|GetPhysicsConstraint) (Variables|Default|GetBasePlate) "None" (Variables|Default|GetDummy) "None"))